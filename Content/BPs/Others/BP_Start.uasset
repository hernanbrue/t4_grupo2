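; BP_Start marks the level's start point and, on BeginPlay, writes its transform to GM_Hover as the SpawnTransform.
; It then calls BlueSetMessage(true) on every BP_BlueObstacle and BP_RedObstacle, with the red pass nested inside the blue loop.
; A disconnected branch that would set game-only input and spawn the game instance's Character never runs.
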(event `self.ReceiveBeginPlay`
  ;[1 1 1] este funcaba
  (bind _asgm_hover (cast `/Game/BPs/GM_Hover` (`GameplayStatics.GetGameMode`)))
  (set `/Game/BPs/GM_Hover.SpawnTransform` (`self.GetTransform`) _asgm_hover)
  ;[1 1 1] no quitar
  (bind _outactors (`GameplayStatics.GetAllActorsOfClass` "/Game/BPs/BP_BlueObstacle.BP_BlueObstacle_C"))
  (for _array_element _outactors
    (message `/Game/BPs/Int_Colors.BlueSet` _array_element true)
    (bind _outactors_2 (`GameplayStatics.GetAllActorsOfClass` "/Game/BPs/BP_RedObstacle.BP_RedObstacle_C"))
    (for _array_element_2 _outactors_2
      (message `/Game/BPs/Int_Colors.BlueSet` _array_element_2 true))))

(fn `UserConstructionScript`)