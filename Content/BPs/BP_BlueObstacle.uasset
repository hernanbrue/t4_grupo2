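; BP_BlueObstacle is an obstacle Actor whose static mesh loses collision while IsBlue is true.
; Every Tick it switches the mesh between NoCollision and QueryAndPhysics based on that flag.
; Collider overlaps with Player-tagged actors toggle IsBlueLeft, which nothing in these graphs reads.
; The BlueSet event is empty, and a half-second Delay before re-enabling collision is disconnected.
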(event `self.ReceiveBeginPlay`
  (set `self.isBlueLeft` true)
  (`PrimitiveComponent.SetCollisionEnabled` (`self.StaticMesh`) "QueryAndPhysics"))

(event `self.Collider.OnComponentBeginOverlap`
  (params (OverlappedComponent :type "PrimitiveComponent Object Reference") (OtherActor :type "Actor Object Reference") (OtherComp :type "PrimitiveComponent Object Reference") (OtherBodyIndex :type Integer) (bFromSweep :type Boolean) (SweepResult :type "HitResult Structure (by ref)"))
  (if (`self.ActorHasTag` OtherActor "Player")
    (set `self.isBlueLeft` false)))

(event `self.Collider.OnComponentEndOverlap`
  (params (OverlappedComponent :type "PrimitiveComponent Object Reference") (OtherActor :type "Actor Object Reference") (OtherComp :type "PrimitiveComponent Object Reference") (OtherBodyIndex :type Integer))
  (if (`self.ActorHasTag` OtherActor "Player")
    (set `self.isBlueLeft` true)))

(event `self.ReceiveTick`
  (params (DeltaSeconds :type "Float (single-precision)"))
  (bind _staticmesh (`self.StaticMesh`))
  (if (stale `/Game/BPs/Int_Colors.BlueSet` isBlue)
    (`PrimitiveComponent.SetCollisionEnabled` _staticmesh "NoCollision")
    (else
      (`PrimitiveComponent.SetCollisionEnabled` _staticmesh "QueryAndPhysics"))))

(event `/Game/BPs/Int_Colors.BlueSet`
  (params (isBlue :type Boolean)))

(fn `UserConstructionScript`)