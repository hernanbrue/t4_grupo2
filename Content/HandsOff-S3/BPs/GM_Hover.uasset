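; Hover racing game mode that spawns the player's car and respawns it when destroyed.
; BeginPlay messages the red and blue obstacles, then spawns and possesses a BP_HoverPawn using the mesh chosen in CARS_GameInstance.
; A destroyed-event binding spawns and possesses a replacement at SpawnTransform, then rebinds.
; Ghost functions record, save, load and replay transform, thrust and steering, but their setup is disconnected and Tick is empty.
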(event `Respawn`
  (bind _asbp_hover_pawn (cast `/Game/HandsOff-S3/BPs/HoverVehicle/BP_HoverPawn` (`GameplayStatics.GetPlayerPawn` 0) :!label _label))
  (`/Engine/EditorBlueprintResources/StandardMacros.IsValid` _asbp_hover_pawn
    (:`Is Valid`
      (add `self.OnDestroyed` _asbp_hover_pawn (delegate `OnCarDestroyed`)))))

(event `self.ReceiveBeginPlay`
  ;[1 1 1] NO QUITAR
  (bind _outactors (`GameplayStatics.GetAllActorsOfClass` "/Game/HandsOff-S3/BPs/BP_BlueObstacle.BP_BlueObstacle_C"))
  (for _array_element _outactors
    _)
  (message `/Game/HandsOff-S3/BPs/Int_Colors.BlueSet` _array_element true)
  (bind _outactors_2 (`GameplayStatics.GetAllActorsOfClass` "/Game/HandsOff-S3/BPs/BP_RedObstacle.BP_RedObstacle_C"))
  (for _array_element_2 _outactors_2
    _)
  (message `/Game/HandsOff-S3/BPs/Int_Colors.BlueSet` _array_element_2 true)
  (bind _returnvalue (`self.SpawnCar` (`self.SpawnTransform`)))
  (`Controller.Possess` (`GameplayStatics.GetPlayerController` 0) _returnvalue)
  (goto _label))

(event `OnCarDestroyed` :!signature `self.OnDestroyed`
  (params (DestroyedActor :type "Actor Object Reference"))
  (bind _spawntransform (`self.SpawnTransform`))
  ;[1 1 1] Respawn
  (bind _returnvalue (`self.SpawnCar` _spawntransform))
  (`KismetSystemLibrary.PrintString` (`KismetStringLibrary.Concat_StrStr` "Spawned " (`KismetSystemLibrary.GetDisplayName` _returnvalue) " in " (`KismetStringLibrary.Conv_TransformToString` _spawntransform)))
  (`KismetSystemLibrary.Delay` 0.2)
  (`Controller.Possess` (`GameplayStatics.GetPlayerController` 0) _returnvalue)
  (`self.Respawn`))

(event `self.ReceiveTick`
  (params (DeltaSeconds :type "Float (single-precision)"))
  ;[1 1 1] Para el ghost
)

(event `OpenGate`
  ;[1 1 1] Para el ghost
  (`/Engine/EditorBlueprintResources/StandardMacros.Gate` true :!via `Open`
    (:`Exit`
      (`self.RecordGhost`)
      (`self.ReplayGhost`))))

(fn `LoadGame`
  (returns (True :type Boolean))
  (bind _returnvalue (`GameplayStatics.DoesSaveGameExist` (`self.SaveGameSlotName`)))
  (if _returnvalue
    (bind _returnvalue_2 (`GameplayStatics.LoadGameFromSlot` (`self.SaveGameSlotName`)))
    (bind _asbp_save_ghost (cast `/Game/HandsOff-S3/BPs/Ghost/BP_SaveGhost` _returnvalue_2)
      (:`then`
        (set `self.GhostInfoReplay` (`/Game/HandsOff-S3/BPs/Ghost/BP_SaveGhost.CarInfoArray` _asbp_save_ghost)))
      (:`CastFailed`
        _)))
  (return _returnvalue))

(fn `RecordGhost`
  (bind _playerpawn (`self.PlayerPawn`))
  (`KismetArrayLibrary.Array_Add` (`self.GhostInfoRecord`) (make `/Game/HandsOff-S3/BPs/Ghost/BP_GhostStruct` (`SceneComponent.K2_GetComponentToWorld` (`/Game/HandsOff-S3/BPs/HoverVehicle/BP_HoverPawn.Body` _playerpawn)) (`/Game/HandsOff-S3/BPs/HoverVehicle/BP_HoverPawn.ThrustGhost` _playerpawn) (`/Game/HandsOff-S3/BPs/HoverVehicle/BP_HoverPawn.SteeringGhost` _playerpawn))))

(fn `ReplayGhost`
  (bind _ghostpawn (`self.GhostPawn`))
  (bind (_output_transform _output_forwardforce _output_steering) (break `/Game/HandsOff-S3/BPs/Ghost/BP_GhostStruct` (`|GetArrayItem` (`self.GhostInfoReplay`) (`self.index`))))
  (set `self.index` (+ (`self.index`) 1))
  (`|ExecutionSequence`
    (:`then_0`
      (`SceneComponent.K2_SetWorldTransform` (`/Game/HandsOff-S3/BPs/HoverVehicle/BP_HoverPawn.Body` _ghostpawn) _output_transform false true))
    (:`then_1`
      (set `/Game/HandsOff-S3/BPs/HoverVehicle/BP_HoverPawn.ThrustGhost` _output_forwardforce _ghostpawn))
    (:`then_2`
      (set `/Game/HandsOff-S3/BPs/HoverVehicle/BP_HoverPawn.SteeringGhost` _output_steering _ghostpawn))))

(fn `SaveGame`
  (`/Engine/EditorBlueprintResources/StandardMacros.IsValid` (`self.GhostSaveGameObj`)
    (:`Is Valid`
      (set `/Game/HandsOff-S3/BPs/Ghost/BP_SaveGhost.CarInfoArray` (`self.GhostInfoRecord`) (stale _output_get))
      (bind _returnvalue (`GameplayStatics.SaveGameToSlot` (`self.GhostSaveGameObj`) (`self.SaveGameSlotName`)))
      (if _returnvalue
        (`KismetSystemLibrary.PrintString` "SAVED!" true true (struct :`R` 1.0 :`G` 0.028454 :`A` 1.0))
        (else
          (`KismetSystemLibrary.PrintString` "NOT SAVED!" true true (struct :`R` 1.0 :`G` 0.028454 :`A` 1.0)))))
    (:`Is Not Valid`
      (bind _returnvalue_2 (`GameplayStatics.CreateSaveGameObject` "/Game/HandsOff-S3/BPs/Ghost/BP_SaveGhost.BP_SaveGhost_C"))
      (bind _output_get (set `self.GhostSaveGameObj` _returnvalue_2)))))

(fn `SpawnCar`
  (params (SpawnTransform :type "Transform Structure"))
  (returns (ReturnValue :type "/Game/HandsOff-S3/BPs/HoverVehicle/BP_HoverPawn Object Reference"))
  (bind _returnvalue (`|SpawnActorFromClass` "/Game/HandsOff-S3/BPs/HoverVehicle/BP_HoverPawn.BP_HoverPawn_C" SpawnTransform "AdjustIfPossibleButAlwaysSpawn" "OverrideRootScale" null null))
  (`/Engine/EditorBlueprintResources/StandardMacros.IsValid` _returnvalue
    (:`Is Valid`
      (bind _ascars_game_instance (cast `/Game/HandsOff-S3/BPs/CARS_GameInstance` (`GameplayStatics.GetGameInstance`)))
      (`StaticMeshComponent.SetStaticMesh` (`/Game/HandsOff-S3/BPs/HoverVehicle/BP_HoverPawn.StaticMesh` _returnvalue) (`/Game/HandsOff-S3/BPs/CARS_GameInstance.Car` _ascars_game_instance))
      (return _returnvalue))
    (:`Is Not Valid`
      (`KismetSystemLibrary.PrintString` "not valid oopsie doopsie"))))

(fn `SpawnGhost`
  (params (`True?` :type Boolean))
  (if `True?`
    (bind _returnvalue (`|SpawnActorFromClass` "/Game/HandsOff-S3/BPs/Ghost/BP_HoverGhost.BP_HoverGhost_C" (`SceneComponent.K2_GetComponentToWorld` (`/Game/HandsOff-S3/BPs/HoverVehicle/BP_HoverPawn.Body` (`self.PlayerPawn`))) "AlwaysSpawn" "OverrideRootScale" null null))
    (set `self.GhostPawn` _returnvalue)))

(fn `UserConstructionScript`)