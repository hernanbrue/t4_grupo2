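; BP_lightRed is a pulsing light Blueprint that makes its light flicker rapidly in the level.
; On BeginPlay it stores the Light component's intensity as MaxPower.
; Each tick it sets the intensity to a fast sine of game time scaled by MaxPower, so the negative half of each wave also feeds into SetIntensity.
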(event `self.ReceiveBeginPlay`
  (set `self.MaxPower` (`LightComponentBase.Intensity` (`self.Light`))))

(event `self.ReceiveTick`
  (params (DeltaSeconds :type "Float (single-precision)"))
  (`LightComponent.SetIntensity` (`self.Light`) (* (`KismetMathLibrary.Sin` (* (`KismetSystemLibrary.GetGameTimeInSeconds`) 10.0)) (`self.MaxPower`))))

(fn `UserConstructionScript`)