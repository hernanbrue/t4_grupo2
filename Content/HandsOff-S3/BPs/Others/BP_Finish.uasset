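; BP_Finish is the finish-line actor that counts laps and decides the race result in what appears to be a hover racing game.
; Each overlap, with no filter on the overlapping actor, increments LapCounter until MaxLaps is reached.
; A later overlap compares GM_Hover's ActualTime to BestLapTime, which resets to a fixed target on BeginPlay.
; Slower runs show WP_FailMenu; others save BestT to CARS_GameInstance and show WP_WinMenu, both with mouse cursor.
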(event `self.ReceiveBeginPlay`
  (bind _output_get (set `self.Best Lap Time` 100.0)))

(event `self.ReceiveActorBeginOverlap`
  (params (OtherActor :type "Actor Object Reference"))
  (bind _asgm_hover (cast `/Game/HandsOff-S3/BPs/GM_Hover` (`GameplayStatics.GetGameMode`)))
  (if (< (`self.LapCounter`) (`self.MaxLaps`))
    (set `self.LapCounter` (+ (`self.LapCounter`) 1))
    (`KismetSystemLibrary.PrintString` "vuelta mas")
    (else
      (`KismetSystemLibrary.PrintString` "FIN")
      (bind _actualtime (`/Game/HandsOff-S3/BPs/GM_Hover.ActualTime` _asgm_hover))
      (if (> _actualtime (stale `self.ReceiveBeginPlay` _output_get))
        (`KismetSystemLibrary.PrintString` "NO SUPERASTE")
        (bind _returnvalue (`|CreateWidget` "/Game/HandsOff-S3/BPs/MainMenu/WP_FailMenu.WP_FailMenu_C"))
        (`UserWidget.AddToViewport` _returnvalue 0)
        (set `PlayerController.bShowMouseCursor` true (`GameplayStatics.GetPlayerController` 0))
        (else
          (bind _output_get (set `self.Best Lap Time` _actualtime))
          (`KismetSystemLibrary.PrintString` "MEJOR TIEMPO")
          (bind _ascars_game_instance (cast `/Game/HandsOff-S3/BPs/CARS_GameInstance` (`GameplayStatics.GetGameInstance`)))
          (set `/Game/HandsOff-S3/BPs/CARS_GameInstance.BestT` _output_get _ascars_game_instance)
          (bind _returnvalue_2 (`|CreateWidget` "/Game/HandsOff-S3/BPs/MainMenu/WP_WinMenu.WP_WinMenu_C"))
          (`UserWidget.AddToViewport` _returnvalue_2 0)
          (set `PlayerController.bShowMouseCursor` true (`GameplayStatics.GetPlayerController` 0)))))))

(fn `UserConstructionScript`)