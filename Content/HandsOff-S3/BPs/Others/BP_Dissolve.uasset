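; BP_Dissolve drives a dissolve fade tied to the player pawn's remaining lifespan.
; On BeginPlay it creates and stores a dynamic instance of the dissolve material, which the graph never uses afterward.
; Each Tick maps the pawn's remaining-to-initial lifespan ratio to a clamped value that rises as life runs out, writes it to the Fade parameter of a Material Parameter Collection, and prints it.
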(event `self.ReceiveBeginPlay`
  (bind _returnvalue (`KismetMaterialLibrary.CreateDynamicMaterialInstance` "/Game/HandsOff-S3/Assets/Arte3D/Meshes/Hover/materiales/MaterialDissolve_Inst.MaterialDissolve_Inst" "None"))
  (set `self.Dissolve` _returnvalue))

(event `self.ReceiveTick`
  (params (DeltaSeconds :type "Float (single-precision)"))
  (bind _returnvalue (`GameplayStatics.GetPlayerPawn` 0))
  (bind _returnvalue_2 (`KismetMathLibrary.MapRangeClamped` (/ (`self.GetLifeSpan` _returnvalue) (`Actor.InitialLifeSpan` _returnvalue)) 1.0 0.1 0.0 8.0))
  (`KismetMaterialLibrary.SetScalarParameterValue` (`self.Collection`) (`self.Fade`) _returnvalue_2)
  (`KismetSystemLibrary.PrintString` (`KismetStringLibrary.Conv_DoubleToString` _returnvalue_2)))

(fn `UserConstructionScript`)