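; BP_BlueObstacle is a color-gate obstacle for the hover pawn, with mesh collision disabled and a Collider detecting overlaps.
; On overlap, a Player-tagged actor while the pawn's ColorSet is the first enum value counts as wrong color.
; That penalty shortens the pawn's actor lifespan, used as a countdown, and triggers camera shake, sound and metal destruction particles.
; When the player exits, it sets IsBlueLeft; other outcomes only print debug text.
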(event `self.ReceiveBeginPlay`
  (`PrimitiveComponent.SetCollisionEnabled` (`self.StaticMesh`) "NoCollision"))

(event `self.Collider.OnComponentEndOverlap`
  (params (OverlappedComponent :type "PrimitiveComponent Object Reference") (OtherActor :type "Actor Object Reference") (OtherComp :type "PrimitiveComponent Object Reference") (OtherBodyIndex :type Integer))
  (if (`self.ActorHasTag` OtherActor "Player")
    (set `self.isBlueLeft` true)))

(event `self.Collider.OnComponentBeginOverlap`
  (params (OverlappedComponent :type "PrimitiveComponent Object Reference") (OtherActor :type "Actor Object Reference") (OtherComp :type "PrimitiveComponent Object Reference") (OtherBodyIndex :type Integer) (bFromSweep :type Boolean) (SweepResult :type "HitResult Structure (by ref)"))
  (bind _asbp_hover_pawn (cast `/Game/HandsOff-S3/BPs/HoverVehicle/BP_HoverPawn` (`GameplayStatics.GetPlayerPawn` 0)))
  (if (and (`self.ActorHasTag` OtherActor "Player") (`|EnumEquality` (`/Game/HandsOff-S3/BPs/HoverVehicle/BP_HoverPawn.ColorSet` _asbp_hover_pawn) "NewEnumerator0"))
    (`KismetSystemLibrary.PrintString` "MAL COLOR")
    (`self.SetLifeSpan` _asbp_hover_pawn (- (`self.GetLifeSpan` _asbp_hover_pawn) 2.0))
    (`MatineeCameraShake.StartMatineeCameraShake` (`GameplayStatics.GetPlayerCameraManager` 0) "/Game/HandsOff-S3/BPs/BP_CameraShake.BP_CameraShake_C")
    (`GameplayStatics.PlaySound2D` "/Game/MusicandSFX/FX/WRONG_Cue.WRONG_Cue" 1.0 1.0 0.0 null null)
    (`ActorComponent.SetActive` (`/Game/HandsOff-S3/BPs/HoverVehicle/BP_HoverPawn.P_Destruction_Metal` _asbp_hover_pawn) true false)
    (`ActorComponent.SetActive` (`/Game/HandsOff-S3/BPs/HoverVehicle/BP_HoverPawn.P_Destruction_Metal1` _asbp_hover_pawn) true false)
    (else
      (`KismetSystemLibrary.PrintString` "BIEN COLOR"))))

(fn `UserConstructionScript`)