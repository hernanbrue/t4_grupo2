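; BP_LateralStabilizer is a component in the hover vehicle folder that damps sideways drift of its owning actor's physics body.
; On BeginPlay it caches the owner's root primitive component.
; Each tick it projects linear velocity onto the body's right vector and applies an opposing force along that axis, proportional to lateral speed and scaled by SpeedToForceFactor.
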(event `self.ReceiveBeginPlay`
  (bind _asprimitive_component (cast `PrimitiveComponent` (`Actor.RootComponent` (`self.GetOwner`))))
  (set `self.Ref to Body` _asprimitive_component))

(event `self.ReceiveTick`
  (params (DeltaSeconds :type "Float (single-precision)"))
  (bind _ref_to_body (`self.Ref to Body`))
  (bind _ref_to_body_2 (`self.Ref to Body`)
    (:`then`
      (bind _returnvalue (`PrimitiveComponent.GetPhysicsLinearVelocity` _ref_to_body_2 "None"))
      (`PrimitiveComponent.AddForce` _ref_to_body (* (`SceneComponent.GetRightVector` _ref_to_body) (* (`KismetMathLibrary.Dot_VectorVector` _returnvalue (`SceneComponent.GetRightVector` _ref_to_body_2)) -10.0 (`self.SpeedToForceFactor`))) "None" false))
    (:`else`)))