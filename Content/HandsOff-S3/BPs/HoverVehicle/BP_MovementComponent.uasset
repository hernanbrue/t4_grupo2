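; Movement component for a hover vehicle that drives the owner's physics body toward a target forward speed and yaw rate.
; On BeginPlay it caches the owner's root primitive component.
; Each tick it measures velocity along the body's forward and up axes, then applies force and torque proportional to the speed errors, acting as a simple P-controller.
; Target speeds are only read here, and hover lift is not handled.
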(event `self.ReceiveBeginPlay`
  (bind _asprimitive_component (cast `PrimitiveComponent` (`Actor.RootComponent` (`self.GetOwner`))))
  (set `self.Ref To Body` _asprimitive_component))

(event `self.ReceiveTick`
  (params (DeltaSeconds :type "Float (single-precision)"))
  (bind _ref_to_body (`self.Ref To Body`))
  (bind _ref_to_body_2 (`self.Ref To Body`))
  (bind _ref_to_body_3 (`self.Ref To Body`))
  (bind _ref_to_body_4 (`self.Ref To Body`)
    (:`then`
      (bind _returnvalue (`PrimitiveComponent.GetPhysicsLinearVelocity` _ref_to_body_4 "None"))
      (set `self.CurrentSpeed` (`KismetMathLibrary.Dot_VectorVector` _returnvalue (`SceneComponent.GetForwardVector` _ref_to_body_4)))
      (set `self.CurrentngularSpeed` (`KismetMathLibrary.Dot_VectorVector` (`PrimitiveComponent.GetPhysicsAngularVelocityInDegrees` _ref_to_body "None") (`SceneComponent.GetUpVector` _ref_to_body)))
      (`PrimitiveComponent.AddForce` _ref_to_body_2 (* (`KismetMathLibrary.MakeVector` (.x (`SceneComponent.GetForwardVector` _ref_to_body_2)) (.y (`SceneComponent.GetForwardVector` _ref_to_body_2)) (.z (`SceneComponent.GetForwardVector` _ref_to_body_2))) (`KismetMathLibrary.Conv_DoubleToVector` (* (- (`self.TargetSpeed`) (`self.CurrentSpeed`)) (`self.Speed To Force Factor`)))) "None" false)
      (`PrimitiveComponent.AddTorqueInDegrees` _ref_to_body_3 (* (`KismetMathLibrary.MakeVector` (.x (`SceneComponent.GetUpVector` _ref_to_body_3)) (.y (`SceneComponent.GetUpVector` _ref_to_body_3)) (.z (`SceneComponent.GetUpVector` _ref_to_body_3))) (`KismetMathLibrary.Conv_DoubleToVector` (* (- (`self.Target AngularSpeed`) (`self.CurrentngularSpeed`)) (`self.Angular Speed To Torque Factor`)))) "None" false))
    (:`else`)))