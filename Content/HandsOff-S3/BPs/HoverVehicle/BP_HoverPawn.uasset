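; Player hover-vehicle pawn for a racing game, with boost, red/blue color switching and a start countdown.
; Tick advances GM_Hover's timer and traces below the body to apply custom gravity, while losing ground triggers a delayed destroy and respawn from the game mode.
; Input feeds the movement component's target speeds, scaled for thrust by boost, ground contact and color-dependent BlueRamp overlaps.
; Gravity flip, red ramp and obstacle toggling logic is disconnected.
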(event `self.ReceiveTick`
  (params (DeltaSeconds :type "Float (single-precision)"))
  (bind _body (`self.Body`))
  (bind _springarm (`self.SpringArm`))
  (bind _body_2 (`self.Body`))
  (bind _rotate (`self.Rotate`))
  (bind _returnvalue (`SceneComponent.K2_GetComponentLocation` _rotate))
  (bind _returnvalue_2 (`SceneComponent.K2_GetComponentLocation` _body_2))
  ;[1 1 1] Initial Life Span
  (if (> (`self.GetLifeSpan`) 0.1)
    (if (or (`self.IsOnGround`) (`self.Flipped`))
      (set `SpringArmComponent.bInheritRoll` true _springarm)
      (set `SpringArmComponent.bInheritPitch` true _springarm)
      (else
        (set `SpringArmComponent.bInheritRoll` false _springarm)
        (set `SpringArmComponent.bInheritPitch` false _springarm)))
    (bind _asgm_hover (cast `/Game/HandsOff-S3/BPs/GM_Hover` (`GameplayStatics.GetGameMode`)))
    (set `/Game/HandsOff-S3/BPs/GM_Hover.ActualTime` (+ DeltaSeconds (`/Game/HandsOff-S3/BPs/GM_Hover.ActualTime` _asgm_hover)) _asgm_hover)
    ;[1 1 1] raycasting
    (bind (_outhit _returnvalue_3) (`KismetSystemLibrary.LineTraceSingle` _returnvalue_2 (- _returnvalue_2 (* (`SceneComponent.GetUpVector` _body_2) 500.0)) "TraceTypeQuery1" false (`|MakeArray` (`self.GetOwner`)) "None" true (struct :`R` 1.0 :`B` 0.935633 :`A` 1.0)))
    (bind _output_get (set `self.IsOnGround` _returnvalue_3))
    (if _output_get
      (`GameplayStatics.PlaySound2D` (`self.HoverSound`) 0.1 1.0 0.0 null null)
      ;[1 1 1] Explicación: si canBoost est'a en azul, entonces dependiendo de su color activo o no la gravedad perpendicular a su body y de esa manera evito que trepe obstáculos. Creo que funca
      (if (`self.canBoost?`)
        (`KismetSystemLibrary.LineTraceSingle` :`Start` _returnvalue :`End` (- _returnvalue (* (`SceneComponent.GetUpVector` _rotate) 500.0)) :`TraceChannel` "TraceTypeQuery1" :`TraceColor` (struct :`R` 1.0 :`B` 0.935633 :`A` 1.0))
        ;[1 1 1] fisicas de gravedad
        (`PrimitiveComponent.AddForce` _body (* (`SceneComponent.GetUpVector` _body) (`self.Gravity`)) "None" true)
        (else
          (`KismetSystemLibrary.Delay` 3.0)
          (`KismetSystemLibrary.Delay` 0.2)
          (`PrimitiveComponent.AddForce` _body (* (* (`KismetMathLibrary.GetUpVector` (struct)) (`self.Gravity`)) 60.0) "None" true)))
      (else
        (`KismetSystemLibrary.Delay` 2.0)
        (`self.K2_DestroyActor`)
        (bind _asgm_hover_2 (cast `/Game/HandsOff-S3/BPs/GM_Hover` (`GameplayStatics.GetGameMode`)))
        (`|SpawnActorFromClass` (`GameplayStatics.GetObjectClass` (`/Game/HandsOff-S3/BPs/GM_Hover.PlayerPawn` _asgm_hover_2)) (`/Game/HandsOff-S3/BPs/GM_Hover.SpawnTransform` _asgm_hover_2) "AlwaysSpawn" "OverrideRootScale" null null)))
    (else
      (`self.K2_DestroyActor`))))

(event `InputAction|Boost`
  (params (Key :type "Key Structure"))
  ;[1 1 1] BOOST
  (:`Pressed`
    (set `self.BoostActive?` true)
    (`GameplayStatics.PlaySound2D` "/Game/MusicandSFX/FX/nitro_Cue.nitro_Cue" 1.0 1.0 0.0 null null)
    (`ActorComponent.Activate` (`self.ShockWave`) false)
    (`ActorComponent.Activate` (`self.NS_Projectile3_Small`) false)
    (set `self.BoostMultiplier` 2.0)
    (`CameraComponent.SetFieldOfView` (`self.Camera`) (`KismetMathLibrary.FInterpTo` (`CameraComponent.FieldOfView` (`self.Camera`)) 120.0 (`GameplayStatics.GetWorldDeltaSeconds`) 0.1))
    (`KismetSystemLibrary.Delay` (`self.BoostDuration`))
    (set `self.BoostMultiplier` 1.0)
    (`CameraComponent.SetFieldOfView` (`self.Camera`) (`KismetMathLibrary.FInterpTo` (`CameraComponent.FieldOfView` (`self.Camera`)) 90.0 (`GameplayStatics.GetWorldDeltaSeconds`) 0.1))
    (`ActorComponent.Deactivate` (`self.ShockWave`))
    (`ActorComponent.Deactivate` (`self.NS_Projectile3_Small`)))
  (:`Released`
    (set `self.BoostActive?` false)))

(event `InputAction|Destroy`
  (params (Key :type "Key Structure"))
  ;[1 1 1] BOOST
  (:`Pressed`
    (`self.K2_DestroyActor`)))

(event `self.ReceiveBeginPlay`
  (bind _asgm_hover (cast `/Game/HandsOff-S3/BPs/GM_Hover` (`GameplayStatics.GetGameMode`)))
  (set `self.As GM Hover` _asgm_hover)
  (set `self.canBoost?` true)
  (set `self.ColorSet` "NewEnumerator1")
  (set `self.BoostMultiplier` 1.0)
  (set `self.isUp` false)
  (`PrimitiveComponent.SetEnableGravity` (`self.Body`) false)
  ;[0.3176 0.102 1] Crear widget 3 2 1
  (if (not (`/Game/HandsOff-S3/BPs/GM_Hover.IsSpawn` (`self.As GM Hover`)))
    (`/Engine/EditorBlueprintResources/StandardMacros.DoOnce` false
      (:`Completed`
        (bind _returnvalue (`GameplayStatics.GetCurrentLevelName` true))
        (if (not (or (`KismetStringLibrary.EqualEqual_StrStr` _returnvalue "Intro") (`KismetStringLibrary.EqualEqual_StrStr` _returnvalue "CarSelection") (`KismetStringLibrary.EqualEqual_StrStr` _returnvalue "MainMenu")))
          (bind _returnvalue_2 (`|CreateWidget` "/Game/HandsOff-S3/BPs/Widgets/321StarWidget.321StarWidget_C"))
          (bind _output_get (set `self.widgetStart` _returnvalue_2))
          (`UserWidget.AddToViewport` _returnvalue_2 0)
          (`UserWidget.AddToViewport` _output_get 0)
          (`KismetSystemLibrary.Delay` 4.0)
          (set `self.start?` false)
          (`Widget.RemoveFromParent` (`self.widgetStart`))
          (set `/Game/HandsOff-S3/BPs/GM_Hover.IsSpawn` true (`self.As GM Hover`)))))))

(event `InputAxis|Thrust`
  (params (AxisValue :type "Float (single-precision)"))
  (bind _movementcomponent (`self.MovementComponent`))
  (bind _returnvalue (* AxisValue (`self.ThrustForce`) (`self.BoostMultiplier`) (`self.BoostRamp`) 1.0))
  ;[0.3176 0.102 1] Movimiento Auto
  (if (`/Game/HandsOff-S3/BPs/GM_Hover.IsSpawn` (`self.As GM Hover`))
    (set `self.ThrustGhost` _returnvalue)
    (if (`self.IsOnGround`)
      (set `/Game/HandsOff-S3/BPs/HoverVehicle/BP_MovementComponent.TargetSpeed` _returnvalue _movementcomponent)
      (else
        (set `/Game/HandsOff-S3/BPs/HoverVehicle/BP_MovementComponent.TargetSpeed` (* _returnvalue 0.2) _movementcomponent)))))

(event `self.Body.OnComponentBeginOverlap`
  (params (OverlappedComponent :type "PrimitiveComponent Object Reference") (OtherActor :type "Actor Object Reference") (OtherComp :type "PrimitiveComponent Object Reference") (OtherBodyIndex :type Integer) (bFromSweep :type Boolean) (SweepResult :type "HitResult Structure (by ref)"))
  (bind _shockwave (`self.ShockWave`))
  ;[1 1 1] ramps
  (if (`self.ActorHasTag` OtherActor "BlueRamp")
    (if (`|EnumEquality` (`self.ColorSet`) "NewEnumerator1")
      (set `self.BoostRamp` 5.0)
      (`ActorComponent.SetActive` _shockwave true false)
      (`KismetSystemLibrary.Delay` 1.5)
      (`ActorComponent.SetActive` _shockwave false false)
      (else
        (set `self.BoostRamp` 0.5)))
    (else
      (set `self.BoostRamp` 1.0))))

(event `self.ReceiveActorEndOverlap`
  (params (OtherActor :type "Actor Object Reference"))
  ;[1 1 1] ramps
  (if (`self.ActorHasTag` OtherActor "BlueRamp")
    (set `self.BoostRamp` 1.0)))

(event `InputAxis|Steer`
  (params (AxisValue :type "Float (single-precision)"))
  ;[1 1 1] LA PRIMERA PARTE ES PARA ADAPTAR EL STEER EN FUNCIÓN A VELOCIDAD
  ;;[1 1 1] modificación del steer
  (set `/Game/HandsOff-S3/BPs/HoverVehicle/BP_MovementComponent.Target AngularSpeed` (* AxisValue 250.0 1.0) (`self.MovementComponent`)))

(event `InputAction|ChangeColor`
  (params (Key :type "Key Structure"))
  (bind _ns_projectile3_small (`self.NS_Projectile3_Small`))
  (bind _flotar1 (`self.Flotar1`))
  (bind _staticmesh (`self.StaticMesh`))
  ;[1 1 1] ColorChange
  (:`Pressed`
    (if (`|EnumEquality` (`self.ColorSet`) "NewEnumerator1")
      (`PrimitiveComponent.SetMaterialByName` _staticmesh "luz" "/Game/HandsOff-S3/Assets/Arte3D/Meshes/Hover/materiales/emm3.emm3")
      (set `self.ColorSet` "NewEnumerator0")
      (set `self.Color` (struct :`R` 1.0 :`B` 0.032358 :`A` 1.0))
      (`FXSystemComponent.SetColorParameter` _ns_projectile3_small "Color" (struct :`R` 1.0 :`G` 0.153251 :`B` 0.033549 :`A` 1.0))
      (`FXSystemComponent.SetColorParameter` _flotar1 "User_Color" (struct :`R` 1.0 :`G` 0.153251 :`B` 0.033549 :`A` 1.0))
      (`FXSystemComponent.SetColorParameter` (`self.Flotar2`) "User_Color" (struct :`R` 1.0 :`G` 0.153251 :`B` 0.033549 :`A` 1.0))
      (`FXSystemComponent.SetColorParameter` (`self.Flotar3`) "User_Color" (struct :`R` 1.0 :`G` 0.153251 :`B` 0.033549 :`A` 1.0))
      (`FXSystemComponent.SetColorParameter` (`self.Flotar`) "User_Color" (struct :`R` 1.0 :`G` 0.153251 :`B` 0.033549 :`A` 1.0))
      (`GameplayStatics.PlaySound2D` "/Game/MusicandSFX/FX/color_change_Cue.color_change_Cue" 2.0 1.0 0.0 null null)
      (else
        (`PrimitiveComponent.SetMaterialByName` _staticmesh "luz" "/Game/HandsOff-S3/Assets/Arte3D/Meshes/Hover/materiales/emm2.emm2")
        (set `self.ColorSet` "NewEnumerator1")
        (set `self.Color` (struct :`G` 0.013595 :`B` 1.0 :`A` 1.0))
        (`FXSystemComponent.SetColorParameter` _ns_projectile3_small "Color" (struct :`G` 1.0 :`B` 1.0 :`A` 1.0))
        (`FXSystemComponent.SetColorParameter` _flotar1 "User_Color" (struct :`G` 1.0 :`B` 1.0 :`A` 1.0))
        (`FXSystemComponent.SetColorParameter` (`self.Flotar2`) "User_Color" (struct :`G` 1.0 :`B` 1.0 :`A` 1.0))
        (`FXSystemComponent.SetColorParameter` (`self.Flotar3`) "User_Color" (struct :`G` 1.0 :`B` 1.0 :`A` 1.0))
        (`FXSystemComponent.SetColorParameter` (`self.Flotar`) "User_Color" (struct :`G` 1.0 :`B` 1.0 :`A` 1.0))
        (`GameplayStatics.PlaySound2D` "/Game/MusicandSFX/FX/color_change_Cue.color_change_Cue" 2.0 1.0 0.0 null null)))))

(event `InputAction|Flip`
  (params (Key :type "Key Structure"))
  ;[1 0 0] NO FUNCA MAS POR INCOMPATIBILIDAD CON LA MEJORA EN LA CONDUCCIÓN Y LAS FÍSICAS (POR AHORA)
)

(fn `UserConstructionScript`)